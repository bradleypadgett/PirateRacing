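; Ocean actor for the pirate racing game that follows the player to keep water around them.
; The construction script applies a very large uniform scale through the actor transform.
; On BeginPlay it caches the first player's pawn and starts a looping timer that periodically moves the ocean to that pawn's X and Y, avoiding per-tick updates.
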(event Custom|Update%20Ocean
  (bind _player (Variables|Default|GetPlayer)
    (:then
      (Transformation|SetActorLocation (Math|Vector|MakeVector (.x (Transformation|GetActorLocation _player)) (.y (Transformation|GetActorLocation _player)) 0.0) false false))
    (:else)))

(event EventBeginPlay
  (Variables|Default|SetPlayer (Game|Player|GetPlayerPawn 0))
  (Utilities|Time|SetTimerbyFunctionName 0 "Update Ocean" 5.0 true))

(fn ConstructionScript
  (Transformation|SetActorTransform (Math|Transform|MakeTransform "0, 0, 0" "0, 0, 0" (Math|Conversions|ToVector(Float) (Math|Float|MakeLiteralFloat 2.5e+03)))))