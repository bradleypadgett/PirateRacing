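; BP_River is a spline-driven river actor for the pirate racing game, built entirely in the construction script.
; It adds a spline mesh between each pair of spline points, matching positions, tangents and per-point Y/Z scale so width and height follow the spline.
; All segments share one dynamic instance of the river material.
; The first and last segments also set custom primitive data slot 0 to zero, marking the river's ends.
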(event EventBeginPlay)

(event Collision|EventActorBeginOverlap
  (params (OtherActor :type Actor%20Object%20Reference)))

(event EventTick
  (params (DeltaSeconds :type Float%20%28single-precision%29)))

(fn ConstructionScript
  (bind _spline (Variables|Default|GetSpline))
  (bind _returnvalue (Rendering|Material|CreateDynamicMaterialInstance (Variables|Default|GetRiverMaterial) "None" "None" :!class /Script/Engine.KismetMaterialLibrary))
  (Variables|Default|SetRiver%20Material%20Instance _returnvalue)
  (for _index (range 0 (- (Spline|GetNumberOfSplinePoints (Variables|Default|GetSpline)) 2))
    (bind _returnvalue_2 (AddComponent|AddSplineMeshComponent false))
    (SplineMesh|SetForwardAxis _returnvalue_2 "X" true)
    (SplineMesh|SetStartandEnd _returnvalue_2 (Spline|GetLocationatSplinePoint _spline _index "Local") (Spline|GetTangentatSplinePoint _spline _index "Local") (Spline|GetLocationatSplinePoint _spline (+ _index 1) "Local") (Spline|GetTangentatSplinePoint _spline (+ _index 1) "Local") true :!class /Script/Engine.SplineMeshComponent)
    (SplineMesh|SetStartScale _returnvalue_2 (Math|Vector2D|MakeVector2D (.y (Spline|GetScaleatSplinePoint _spline _index)) (.z (Spline|GetScaleatSplinePoint _spline _index))) true :!class /Script/Engine.SplineMeshComponent)
    (SplineMesh|SetEndScale _returnvalue_2 (Math|Vector2D|MakeVector2D (.y (Spline|GetScaleatSplinePoint _spline (+ _index 1))) (.z (Spline|GetScaleatSplinePoint _spline (+ _index 1)))) true :!class /Script/Engine.SplineMeshComponent)
    (Rendering|Material|SetMaterial _returnvalue_2 0 (Variables|Default|GetRiver%20Material%20Instance))
    (if (== _index 0)
      (Rendering|Material|SetCustomPrimitiveDataFloat _returnvalue_2 0 0.0)
      (elif (== _index (- (Spline|GetNumberOfSplinePoints (Variables|Default|GetSpline)) 2))
        (Rendering|Material|SetCustomPrimitiveDataFloat _returnvalue_2 0 0.0)))))