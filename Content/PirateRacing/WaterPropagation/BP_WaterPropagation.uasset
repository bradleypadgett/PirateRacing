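; Water propagation Blueprint that redraws the RT_CollisionInterfaceTrail render target every frame.
; BeginPlay creates a dynamic instance of MI_Test, and Tick draws it across the full canvas without setting any parameters.
; An unconnected fixed-timestep accumulator, driven by UpdateRate with a capped frequency, never runs, so updates follow the frame rate.
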(event EventBeginPlay
  (bind _returnvalue (Rendering|Material|CreateDynamicMaterialInstance "/Game/PirateRacing/WaterPropagation/MI_Test.MI_Test" "None" "None" :!class /Script/Engine.KismetMaterialLibrary))
  (Variables|Default|SetDynamicMaterial _returnvalue))

(event Collision|EventActorBeginOverlap
  (params (OtherActor :type Actor%20Object%20Reference)))

(event EventTick
  (params (DeltaSeconds :type Float%20%28single-precision%29))
  (bind (_canvas _size _context) (Rendering|BeginDrawCanvastoRenderTarget "/Game/PirateRacing/WaterPropagation/RT_CollisionInterfaceTrail.RT_CollisionInterfaceTrail"))
  (Canvas|DrawMaterial :self _canvas :RenderMaterial (Variables|Default|GetDynamicMaterial) :ScreenPosition "(X=0.000000,Y=0.000000)" :ScreenSize _size :CoordinateSize "(X=1.000000,Y=1.000000)" :PivotPoint "(X=0.500000,Y=0.500000)")
  (Rendering|EndDrawCanvastoRenderTarget _context))

(fn ConstructionScript)